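; Game mode for a local two-player épée duel, running a bout of timed rounds with point scoring.
; BeginPlay spawns and possesses fencers at tagged PlayerStarts, cross-links them, creates the HUD and starts the bout.
; Reaching the point limit or leading when final-round time expires wins; ties enter overtime, where a randomly chosen priority player wins on timeout.
; Tick runs the countdown and slows global time whenever either animation blueprint allows a riposte.
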(event `Give Point`
  (params (Player :type "Character Object Reference"))
  (bind _returnvalue (== Player (`self.Player 1`)))
  ;[1 1 1 1 40] Point Scoring
  ;;[0.375 0.75 0.1875] Add one to the scoring player's points
  (if _returnvalue
    (bind _result (`/Engine/EditorBlueprintResources/StandardMacros.IncrementInt` (`self.Player1Points`))
      (:`  `
        _))
    (else
      (bind _result_2 (`/Engine/EditorBlueprintResources/StandardMacros.IncrementInt` (`self.Player2Points`))
        (:`  `
          _))))
  ;;[0.05 0.1 0.1] Update the HUD
  (`/Game/Blueprints/WBP_HUD.UpdateScore` (`self.HUDWidget`) (`self.Player1Points`) (`self.Player2Points`) (`self.OvertimeActive`) (`self.PriorityPlayer`))
  (`/Game/Blueprints/WBP_HUD.Show Touch` (`self.HUDWidget`) Player)
  ;;[0.749 0.6392 0.07451] If the new score is enough to win and the game is still going - End the bout with the scoring player as the winner
  (if (and (>= (`KismetMathLibrary.SelectInt` _result _result_2 _returnvalue) (`self.PointsToWin`)) (not (`self.GameEnded`)))
    (`self.End Bout` Player)))

(event `Overtime Started`
  ;[1 1 1 1 40] Overtime
  ;;[0.375 0.75 0.1875] Restart the timer with a scricter time limit
  (bind _output_get (set `self.Timer` 30.0))
  (`/Game/Blueprints/WBP_HUD.UpdateTimer` (`self.HUDWidget`) _output_get true)
  ;;[0.75 0.075 0.075] Activate Overtime rules and start a new round
  (set `self.OvertimeActive` true)
  (`self.End Round`)
  ;;[0.5625 0.1875 0.75] Pick a random player to have overtime priority
  (bind _output_get_2 (set `self.PriorityPlayer` (select `bool` (`KismetMathLibrary.RandomBool`) :`false` (`self.Player 2`) :`true` (`self.Player 1`))))
  (`/Game/Blueprints/WBP_HUD.UpdateScore` (`self.HUDWidget`) 0 0 true _output_get_2))

(event `self.ReceiveTick`
  (params (DeltaSeconds :type "Float (single-precision)"))
  (bind _returnvalue (- (`self.Timer`) DeltaSeconds))
  ;[1 1 1 1 40] Time
  ;;[0.375 0.1875 0.75] Slow down time while the player can riposte. Makes the timing easier and feels nice
  (`GameplayStatics.SetGlobalTimeDilation` (`KismetMathLibrary.SelectFloat` 0.2 1.0 (or (`/Game/Characters/Mannequins/Animations/ABP_Manny.CanRiposte` (`self.P1ABP`)) (`/Game/Characters/Mannequins/Animations/ABP_Manny.CanRiposte` (`self.P2ABP`)))))
  ;;[0.4688 0.75 0.1875] Have a timer count down each second to 0
  (if (`self.TimerActive`)
    (`/Game/Blueprints/WBP_HUD.UpdateTimer` (`self.HUDWidget`) _returnvalue (`self.OvertimeActive`))
    (if (>= _returnvalue 0.0)
      (set `self.Timer` _returnvalue)
      (else
        ;[0.75 0.1875 0.1875] Once the timer reaches 0, stop and evaluate rules
        (`/Engine/EditorBlueprintResources/StandardMacros.DoOnce` false :!label _label
          (:`Completed`
            (set `self.Timer` 0.0)
            (`self.TimeOver`)))))))

(event `End Round`
  (bind _hudwidget (`self.HUDWidget`))
  ;[1 1 1 1 40] End Round and Bout
  ;;[0.75 0.1875 0.1875] Stop gameplay
  (set `self.TimerActive` false)
  (`self.TogglePlayerControls` false false (`self.Player 1`))
  (`self.TogglePlayerControls` false false (`self.Player 2`))
  (`|ExecutionSequence`
    (:`then_0`
      (goto _label :!via `Reset`))
    (:`then_1`
      ;;[0.05 0.1 0.1] If not the end of the game, play the time-out HUD animation instead of the win animation
      (if (not (`self.GameEnded`))
        (`/Engine/EditorBlueprintResources/StandardMacros.IncrementInt` (`self.CurrentRound`)
          (:`  `
            (`UserWidget.PlayAnimation` _hudwidget (`/Game/Blueprints/WBP_HUD.RoundEndAnim` _hudwidget) 0.0 1 "Forward" 1.0 false)))))))

(event `End Bout`
  (params (Winner :type "Character Object Reference"))
  ;[1 1 1 1 40] End Round and Bout
  (set `self.OvertimeActive` false)
  (set `self.GameEnded` true)
  (`self.End Round`)
  (`/Game/Blueprints/WBP_HUD.Show Win Popup` (`self.HUDWidget`) Winner))

(event `self.ReceiveBeginPlay`
  ;[1 1 1 1 40] BeginPlay
  ;;[0.302 0.07451 0.749] Spawn a new player for each player start on the map
  (bind _outactors (`GameplayStatics.GetAllActorsOfClass` "/Script/Engine.PlayerStart"))
  (for _array_element _outactors
    (`self.SpawnPlayers` _array_element)
    (`KismetSystemLibrary.Delay` 0.1) ; Delay needed because 2nd controller won't work otherwise, UE5 is buggy
    (`self.Possess Players`))
  (`/Engine/EditorBlueprintResources/StandardMacros.IsValid` (`self.Player 1`)
    (:`Is Valid`
      (`/Engine/EditorBlueprintResources/StandardMacros.IsValid` (`self.Player 2`)
        (:`Is Valid`
          ;;[0.1875 0.375 0.75] Give player 1 and 2 references to each other
          (`/Game/Blueprints/BP_GenericEpeeCharacter.AddReferences` (`self.Player 1`) (`self.Player 2`))
          (`/Game/Blueprints/BP_GenericEpeeCharacter.AddReferences` (`self.Player 2`) (`self.Player 1`))
          ;;[0.1875 0.75 0.5625] Save references to animation blueprints
          (bind _asabp_manny (cast `/Game/Characters/Mannequins/Animations/ABP_Manny` (`SkeletalMeshComponent.GetAnimInstance` (`Character.Mesh` (`self.Player 1`)))))
          (set `self.P1ABP` _asabp_manny)
          (bind _asabp_manny_2 (cast `/Game/Characters/Mannequins/Animations/ABP_Manny` (`SkeletalMeshComponent.GetAnimInstance` (`Character.Mesh` (`self.Player 2`)))))
          (set `self.P2ABP` _asabp_manny_2)
          ;;[0.05 0.1 0.1] Spawn HUD
          (bind _returnvalue (`|CreateWidget` "/Game/Blueprints/WBP_HUD.WBP_HUD_C" (`GameplayStatics.GetPlayerController` 0)))
          (bind _output_get (set `self.HUDWidget` _returnvalue))
          (`UserWidget.AddToViewport` _output_get 0)
          ;;[0.05 0.1 0.1] Give the HUD references to each player and us
          (set `/Game/Blueprints/WBP_HUD.Player1` (`self.Player 1`) _output_get)
          (set `/Game/Blueprints/WBP_HUD.Player2` (`self.Player 2`) _output_get)
          (set `/Game/Blueprints/WBP_HUD.Game` self _output_get)
          (`self.Start Bout`))))))

(event `Start Bout`
  ;[1 1 1 1 40] Start Bout
  ;;[0.1875 0.75 0.075] Initialize Game Logic
  (set `self.GameEnded` false)
  (set `self.OvertimeActive` false)
  (set `self.Player1Points` 0)
  (set `self.Player2Points` 0)
  (set `self.CurrentRound` 0)
  (`self.Start Round`))

(event `Enable Gameplay`
  (bind _returnvalue (`GameplayStatics.GetPlayerController` 1))
  (bind _returnvalue_2 (`GameplayStatics.GetPlayerController` 0))
  ;[1 1 1 1 40] Enable Gameplay
  ;;[0.3 0.75 0.075] Turn on player controls and start the timer
  (`self.TogglePlayerControls` true true (`self.Player 1`))
  (`self.TogglePlayerControls` true true (`self.Player 2`))
  (set `self.TimerActive` true)
  (`WidgetBlueprintLibrary.SetInputMode_GameOnly` _returnvalue_2)
  (set `PlayerController.bShowMouseCursor` false _returnvalue_2)
  (`WidgetBlueprintLibrary.SetInputMode_GameOnly` _returnvalue)
  (set `PlayerController.bShowMouseCursor` false _returnvalue))

(event `Start Round`
  (bind _hudwidget (`self.HUDWidget`))
  ;[1 1 1 1 40] Start Round
  ;;[0.302 0.07451 0.749] Reset characters to their original positions
  (`self.ResetPlayerPosition` (`self.Player 1`))
  (`self.ResetPlayerPosition` (`self.Player 2`))
  ;;[0.01569 0.03137 0.03137] Update HUD values and play the startup animation
  (`/Game/Blueprints/WBP_HUD.UpdateScore` (`self.HUDWidget`) (`self.Player1Points`) (`self.Player2Points`) (`self.OvertimeActive`) (`self.PriorityPlayer`))
  (`/Game/Blueprints/WBP_HUD.Update Round` (`self.HUDWidget`) (`self.CurrentRound`) (`self.OvertimeActive`))
  (`UserWidget.PlayAnimation` _hudwidget (`/Game/Blueprints/WBP_HUD.StartAnim` _hudwidget) 0.0 1 "Forward" 1.0 false)
  ;;[0.1875 0.75 0.4688] Reset the timer at the start of a normal round
  (if (not (`self.OvertimeActive`))
    (bind _output_get (set `self.Timer` 75.0))
    (`/Game/Blueprints/WBP_HUD.UpdateTimer` (`self.HUDWidget`) _output_get false)))

(fn `Possess Players`
  (bind _returnvalue (`GameplayStatics.GetPlayerController` 0))
  ;[1 1 1] Possess characters and add mapping contexts to enable control
  (`Controller.Possess` _returnvalue (`self.Player 1`))
  (`EnhancedInputSubsystemInterface.AddMappingContext` (pcsubsystem `EnhancedInputLocalPlayerSubsystem` _returnvalue) "/Game/Input/IMC_Default.IMC_Default" 0 (struct))
  (bind _returnvalue_2 (`GameplayStatics.CreatePlayer` 1))
  (`Controller.Possess` (`GameplayStatics.GetPlayerController` 1) (`self.Player 2`))
  (`EnhancedInputSubsystemInterface.AddMappingContext` (pcsubsystem `EnhancedInputLocalPlayerSubsystem` _returnvalue_2) "/Game/Input/IMC_Default.IMC_Default" 0 (struct)))

(fn `ResetPlayerPosition`
  (params (Player :type "/Game/Blueprints/BP_GenericEpeeCharacter Object Reference"))
  ;[0.75 0.5625 0.1875] Set the player transform to the transform of the player start they were assigned at spawn
  (set `/Game/Blueprints/BP_GenericEpeeCharacter.IsFlipped` false Player)
  (`self.K2_SetActorTransform` Player (`self.GetTransform` (select `bool` (== Player (`self.Player 1`)) :`false` (`self.P2Start`) :`true` (`self.P1Start`))) false true))

(fn `SpawnPlayers`
  (params (Object :type "PlayerStart Object Reference"))
  (bind _playerstarttag (`PlayerStart.PlayerStartTag` Object))
  ;[0.07785 0.2591 1] Detect whether the start point is for player 1 or 2
  (if (== _playerstarttag "P1")
    (bind _output_get (set `self.P1Start` Object))
    (bind _returnvalue (`|SpawnActorFromClass` "/Game/Blueprints/BP_GenericEpeeCharacter.BP_GenericEpeeCharacter_C" (`self.GetTransform` _output_get) "Undefined" "MultiplyWithRoot" _output_get null))
    ;[1 1 1] Assign player references
    (set `self.Player 1` _returnvalue)
    (elif (== _playerstarttag "P2")
      (bind _output_get_2 (set `self.P2Start` Object))
      (bind _returnvalue_2 (`|SpawnActorFromClass` "/Game/Blueprints/BP_GenericEpeeCharacter.BP_GenericEpeeCharacter_C" (`self.GetTransform` Object) "Undefined" "MultiplyWithRoot" _output_get_2 null))
      (set `self.Player 2` _returnvalue_2))))

(fn `TimeOver`
  (bind _player1points (`self.Player1Points`))
  (bind _player2points (`self.Player2Points`))
  ;[0.05 0.05 0.05] Is the bout in overtime?
  (if (`self.OvertimeActive`)
    ;[1 0.702 0.102] End the bout with the winner being the priority player selected at the start of Overtime
    (`self.End Bout` (`self.PriorityPlayer`))
    (else
      ;[0.05 0.05 0.05] Are we on the final round?
      (if (<= (`self.CurrentRound`) 1)
        (`self.End Round`)
        (else
          ;[0.05 0.05 0.05] Is there a clear victor?
          (if (!= _player1points _player2points)
            ;[1 0.702 0.102] End the bout with the winner being the player with the most points
            (`self.End Bout` (select `bool` (> _player1points _player2points) :`false` (`self.Player 2`) :`true` (`self.Player 1`)))
            (else
              (`self.Overtime Started`))))))))

(fn `TogglePlayerControls`
  (params (EnableMovement :type Boolean) (EnableActions :type Boolean) (Player :type "/Game/Blueprints/BP_GenericEpeeCharacter Object Reference"))
  (set `/Game/Blueprints/BP_GenericEpeeCharacter.CanMove` EnableMovement Player)
  (set `/Game/Blueprints/BP_GenericEpeeCharacter.CanAct` EnableActions Player)
  ;[0.75 0.1875 0.1875] Turn any active abilities off if they can't act, for safety
  (if (not EnableActions)
    (set `/Game/Blueprints/BP_GenericEpeeCharacter.AttackActive` false Player)
    (set `/Game/Blueprints/BP_GenericEpeeCharacter.ParryActive` false Player)
    (set `/Game/Blueprints/BP_GenericEpeeCharacter.ParryHit` false Player)))

(fn `UserConstructionScript`)