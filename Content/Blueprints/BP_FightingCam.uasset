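; BP_FightingCam is a fighting-game camera that keeps both duel players in view.
; After a brief delay on BeginPlay, it takes both player references from BP_QuickDuelGameMode and records its starting X.
; Each Tick it centers on the players' Y and backs away along X by their clamped Y separation.
; Its height is the summed player Z over a divisor below two, biasing the view upward.
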(event `self.ReceiveBeginPlay`
  (bind _returnvalue_x (`KismetMathLibrary.BreakVector` (`self.K2_GetActorLocation`)))
  ;[1 1 1] Set References to player characters
  (`KismetSystemLibrary.Delay` 0.03)
  (bind _asbp_third_person_game_mode (cast `/Game/Blueprints/BP_QuickDuelGameMode` (`GameplayStatics.GetGameMode`)))
  (bind _player_1 (`/Game/Blueprints/BP_QuickDuelGameMode.Player 1` _asbp_third_person_game_mode))
  (`/Engine/EditorBlueprintResources/StandardMacros.IsValid` _player_1
    (:`Is Valid`
      (set `self.Player 1 Ref` _player_1)
      (bind _player_2 (`/Game/Blueprints/BP_QuickDuelGameMode.Player 2` _asbp_third_person_game_mode))
      (`/Engine/EditorBlueprintResources/StandardMacros.IsValid` _player_2
        (:`Is Valid`
          (set `self.Player 2 Ref` _player_2)
          (set `self.Initial X Location` _returnvalue_x))))))

(event `self.ReceiveTick`
  (params (DeltaSeconds :type "Float (single-precision)"))
  (bind _player_1_ref (`self.Player 1 Ref`))
  (bind _player_2_ref (`self.Player 2 Ref`))
  (bind (_returnvalue_x _returnvalue_y _returnvalue_z) (`KismetMathLibrary.BreakVector` (`self.K2_GetActorLocation` _player_1_ref)))
  (bind (_returnvalue_x_2 _returnvalue_y_2 _returnvalue_z_2) (`KismetMathLibrary.BreakVector` (`self.K2_GetActorLocation` _player_2_ref)))
  ;[0.05098 0.05098 0.05098] Move the camera to keep both players in view
  (if (and (`KismetSystemLibrary.IsValid` _player_1_ref) (`KismetSystemLibrary.IsValid` _player_2_ref))
    (`self.K2_SetActorLocation` (`KismetMathLibrary.MakeVector` (- (`self.Initial X Location`) (`KismetMathLibrary.FClamp` (`KismetMathLibrary.Abs` (- _returnvalue_y _returnvalue_y_2)) 400.0 1400.0)) (/ (+ _returnvalue_y _returnvalue_y_2) 2.0) (/ (+ _returnvalue_z _returnvalue_z_2) 1.6)))))

(fn `UserConstructionScript`)